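; Instant spell actor that plays cast and impact effects, supporting both Cascade and Niagara assets from its SpellToSpawn data.
; On BeginPlay it attaches the initial cast effect to the player's CastSocket, waits the spell delay, sizes the detection sphere, spawns the cast effect and starts a self-destruct timer.
; Overlapping Enemy-tagged components triggers, after the same delay, an impact effect at the actor's location and a ragdoll hit force on EnemyMesh_BP.
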(event `self.ReceiveBeginPlay`
  (bind _returnvalue (`self.K2_GetActorLocation`))
  (bind _returnvalue_2 (`self.K2_GetActorLocation`))
  (bind _defaultsceneroot (`self.DefaultSceneRoot`))
  (bind _defaultsceneroot_2 (`self.DefaultSceneRoot`))
  (bind ((`Cast_FX_43_5D639F294CD498AA840C339CCC3419D4` _cast_fx) (`InitialCast_FX_46_B58736B241279BFB376B6DBC62E8E8CD` _initialcast_fx) (`ImpactDetectionRadius_28_02EAD3B948868B54081C9CACD01B8260` _impactdetectionradius) (`SpellDelayInSeconds_38_9DBD8B6A4B5FDA2B04E3A0A64CA8D14A` _spelldelayinseconds)) (break `/Game/VFXApprentice/Blueprints/SpellData/InstantSpell_Struct` (`self.SpellToSpawn`)))
  (bind _mesh (`Character.Mesh` (`self.SideScrollerPlayer_BP`)))
  (bind _returnvalue_3 (`SkinnedMeshComponent.GetSocketBoneName` _mesh "CastSocket"))
  (`self.SetSpellTypes`)
  (`/Engine/EditorBlueprintResources/StandardMacros.IsValid` _initialcast_fx
    (:`Is Valid`
      (if (`self.InitialCast_IsStandard?`)
        (bind _returnvalue_4 (`GameplayStatics.SpawnEmitterAttached` (cast `ParticleSystem` _initialcast_fx :!pure true) _defaultsceneroot_2 "None" _returnvalue (struct) (1.0 1.0 1.0) "KeepWorldPosition"))
        (bind _output_get (set `self.WindUpFX` _returnvalue_4))
        (`SceneComponent.K2_AttachToComponent` _output_get _mesh _returnvalue_3 "SnapToTarget" "KeepRelative" "KeepRelative" true)
        (else
          (bind _returnvalue_5 (`NiagaraFunctionLibrary.SpawnSystemAttached` (cast `NiagaraSystem` _initialcast_fx :!pure true) _defaultsceneroot_2 "None" _returnvalue (struct) "KeepWorldPosition" true))
          (bind _output_get_2 (set `self.WindUpFXNiagara` _returnvalue_5))
          (`SceneComponent.K2_AttachToComponent` _output_get_2 _mesh _returnvalue_3 "SnapToTarget" "KeepRelative" "KeepRelative" true)))
      (`KismetSystemLibrary.Delay` _spelldelayinseconds)
      (`SphereComponent.SetSphereRadius` (`self.SpellBounds`) _impactdetectionradius true)
      (`/Engine/EditorBlueprintResources/StandardMacros.IsValid` _cast_fx
        (:`Is Valid`
          (if (`self.Cast_IsStandard?`)
            (bind _returnvalue_6 (`GameplayStatics.SpawnEmitterAttached` (cast `ParticleSystem` _cast_fx :!pure true) _defaultsceneroot "None" _returnvalue_2 (struct) (1.0 1.0 1.0) "KeepWorldPosition"))
            (set `self.SpawnFX` _returnvalue_6)
            (else
              (bind _returnvalue_7 (`NiagaraFunctionLibrary.SpawnSystemAttached` (cast `NiagaraSystem` _cast_fx :!pure true) _defaultsceneroot "None" _returnvalue_2 (struct) "KeepWorldPosition" true))
              (set `self.SpawnFXNiagara` _returnvalue_7)))
          (`KismetSystemLibrary.K2_SetTimerDelegate` (delegate `KillParticle`) (`self.TimeTillDeath`)))))))

(event `KillParticle`
  (set `PrimitiveComponent.bGenerateOverlapEvents` false (`self.SpellBounds`))
  (`self.K2_DestroyActor`))

(event `self.SpellBounds.OnComponentBeginOverlap`
  (params (OverlappedComponent :type "PrimitiveComponent Object Reference") (OtherActor :type "Actor Object Reference") (OtherComp :type "PrimitiveComponent Object Reference") (OtherBodyIndex :type Integer) (bFromSweep :type Boolean) (SweepResult :type "HitResult Structure (by ref)"))
  (bind _returnvalue (`self.K2_GetActorLocation`))
  (bind _defaultsceneroot (`self.DefaultSceneRoot`))
  (bind ((`Impact_FX_44_A51BFC634EE49FB0730E6FAE4CDE912A` _impact_fx) (`SpellDelayInSeconds_38_9DBD8B6A4B5FDA2B04E3A0A64CA8D14A` _spelldelayinseconds) (`RagdollForce_31_96500D8A4E421F879A548792BF8FD33C` _ragdollforce)) (break `/Game/VFXApprentice/Blueprints/SpellData/InstantSpell_Struct` (`self.SpellToSpawn`)))
  ;[1 1 1] Spawn Hit Impact on Enemies
  (`/Engine/EditorBlueprintResources/StandardMacros.IsValid` OtherComp
    (:`Is Valid`
      (if (`ActorComponent.ComponentHasTag` OtherComp "Enemy")
        (`KismetSystemLibrary.Delay` _spelldelayinseconds)
        (if (`self.Impact_IsStandard?`)
          (bind _returnvalue_2 (`GameplayStatics.SpawnEmitterAttached` (cast `ParticleSystem` _impact_fx :!pure true) _defaultsceneroot "None" _returnvalue (struct) (1.0 1.0 1.0) "KeepWorldPosition"))
          (set `self.ImpactFX` _returnvalue_2)
          (else
            (bind _returnvalue_3 (`NiagaraFunctionLibrary.SpawnSystemAttached` (cast `NiagaraSystem` _impact_fx :!pure true) _defaultsceneroot "None" _returnvalue (struct) "KeepWorldPosition" true))
            (set `self.ImpactFXNiagara` _returnvalue_3)))
        (bind _asenemy_mesh_bp (cast `/Game/VFXApprentice/Blueprints/Characters/EnemyMesh_BP` null))
        (`/Game/VFXApprentice/Blueprints/Characters/EnemyMesh_BP.ApplyHitForce` _asenemy_mesh_bp (`SceneComponent.K2_GetComponentLocation` OtherComp) _ragdollforce)))))

(fn `SetSpellTypes`
  (bind ((`Cast_FX_43_5D639F294CD498AA840C339CCC3419D4` _cast_fx) (`Impact_FX_44_A51BFC634EE49FB0730E6FAE4CDE912A` _impact_fx) (`InitialCast_FX_46_B58736B241279BFB376B6DBC62E8E8CD` _initialcast_fx) (`WindUp_FX_47_DF441E3F46C84B5C66DA8B924122F938` _windup_fx)) (break `/Game/VFXApprentice/Blueprints/SpellData/InstantSpell_Struct` (`self.SpellToSpawn`)))
  (set `self.Cast_IsStandard?` (`.bSuccess` (cast `ParticleSystem` _cast_fx :!pure true)))
  (set `self.Impact_IsStandard?` (`.bSuccess` (cast `ParticleSystem` _impact_fx :!pure true)))
  (set `self.InitialCast_IsStandard?` (`.bSuccess` (cast `ParticleSystem` _initialcast_fx :!pure true)))
  (set `self.WindUp_IsStandard?` (`.bSuccess` (cast `ParticleSystem` _windup_fx :!pure true))))

(fn `UserConstructionScript`)