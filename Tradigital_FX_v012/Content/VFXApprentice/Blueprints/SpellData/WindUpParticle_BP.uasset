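; WindUpParticle_BP is an actor that shows a spell's wind-up effect on the player.
; On BeginPlay it attaches to a named socket on the player pawn's mesh, snapping location and keeping relative rotation and scale.
; It then spawns WindUpFX on its root, accepting either a Cascade particle system or a Niagara system, and stores the spawned component.
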(event `self.ReceiveBeginPlay`
  (bind _defaultsceneroot (`self.DefaultSceneRoot`))
  (`self.K2_AttachToComponent` (`Character.Mesh` (`self.PlayerPawn`)) (`self.SocketAttachName`) "SnapToTarget" "KeepRelative" "KeepRelative")
  (bind _asparticle_system (cast `ParticleSystem` (`self.WindUpFX`))
    (:`then`
      (bind _returnvalue (`GameplayStatics.SpawnEmitterAttached` _asparticle_system _defaultsceneroot))
      (set `self.WindUpParticleSystem` _returnvalue))
    (:`CastFailed`
      (bind _asniagara_system (cast `NiagaraSystem` (`self.WindUpFX`)))
      (bind _returnvalue_2 (`NiagaraFunctionLibrary.SpawnSystemAttached` _asniagara_system _defaultsceneroot "None" (0.0 0.0 0.0) (struct) "KeepRelativeOffset" true))
      (set `self.WindUpFXNiagara` _returnvalue_2))))

(event `self.ReceiveTick`
  (params (DeltaSeconds :type "Float (single-precision)")))

(fn `UserConstructionScript`)