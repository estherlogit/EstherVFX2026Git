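; Melee spell actor that plays a cast effect and applies a single hit to an enemy, driven by SpellToSpawn data.
; Its bounds sphere snaps to the SwordCenter socket, then after a spawn delay enables overlaps, resizes, and spawns facing-aware cast FX before timed destruction.
; The first overlap consumes a DoOnce; if enemy-tagged, it applies ragdoll force and impact FX.
; Both effects support either Cascade or Niagara assets.
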(event `self.ReceiveBeginPlay`
  (bind _returnvalue (`self.K2_GetActorLocation`))
  (bind _defaultsceneroot (`self.DefaultSceneRoot`))
  (bind ((`Cast_FX_33_5D639F294CD498AA840C339CCC3419D4` _cast_fx) (`Impact_FX_34_A51BFC634EE49FB0730E6FAE4CDE912A` _impact_fx) (`SpawnDelay_27_8F051FA74AF8C3D166A724A417D34473` _spawndelay) (`ImpactRadius_29_1EF306CB4A14FA7CF1F5C998848AD6FA` _impactradius)) (break `/Game/VFXApprentice/Blueprints/SpellData/MeleeSpell_Struct` (`self.SpellToSpawn`)))
  (bind ((`Cast_FX_33_5D639F294CD498AA840C339CCC3419D4` _cast_fx_2)) (break `/Game/VFXApprentice/Blueprints/SpellData/MeleeSpell_Struct` (`self.SpellToSpawn`)))
  (bind _returnvalue_2 (select `bool` (`/Game/VFXApprentice/Blueprints/Characters/SideScroller_Player_BP.FacingRIght?` (`self.Player Pawn`)) :`false` (struct :`Yaw` 180.0) :!type "Rotator Structure"))
  (`SceneComponent.K2_AttachToComponent` (`self.SpellBounds`) (`self.SkeletalMesh`) "SwordCenter" "SnapToTarget" "KeepRelative" "KeepRelative" true)
  (`KismetSystemLibrary.Delay` _spawndelay)
  (set `PrimitiveComponent.bGenerateOverlapEvents` true (`self.SpellBounds`))
  (`SphereComponent.SetSphereRadius` (`self.SpellBounds`) _impactradius true)
  (bind _asparticle_system (cast `ParticleSystem` _cast_fx_2)
    (:`then`
      (bind _returnvalue_3 (`GameplayStatics.SpawnEmitterAttached` _asparticle_system _defaultsceneroot "None" _returnvalue _returnvalue_2 (1.0 1.0 1.0) "KeepWorldPosition"))
      (set `self.SpawnFX` _returnvalue_3))
    (:`CastFailed`
      (bind _returnvalue_4 (`NiagaraFunctionLibrary.SpawnSystemAttached` (cast `NiagaraSystem` _cast_fx_2 :!pure true) _defaultsceneroot "None" _returnvalue _returnvalue_2 "KeepWorldPosition"))
      (set `self.SpawnFXNIagara` _returnvalue_4)))
  (`KismetSystemLibrary.Delay` (`self.TimeTillDeath`))
  (`self.K2_DestroyActor`))

(event `self.SpellBounds.OnComponentBeginOverlap`
  (params (OverlappedComponent :type "PrimitiveComponent Object Reference") (OtherActor :type "Actor Object Reference") (OtherComp :type "PrimitiveComponent Object Reference") (OtherBodyIndex :type Integer) (bFromSweep :type Boolean) (SweepResult :type "HitResult Structure (by ref)"))
  (bind (_bblockinghit _binitialoverlap _time _distance _location _impactpoint _normal _impactnormal _physmat _hitactor _hitcomponent) (`GameplayStatics.BreakHitResult` SweepResult))
  (bind ((`Cast_FX_33_5D639F294CD498AA840C339CCC3419D4` _cast_fx) (`Impact_FX_34_A51BFC634EE49FB0730E6FAE4CDE912A` _impact_fx) (`RagdollForce_32_8A823B0D49C5814E5F286A8E42F9FBD7` _ragdollforce)) (break `/Game/VFXApprentice/Blueprints/SpellData/MeleeSpell_Struct` (`self.SpellToSpawn`)))
  (bind _returnvalue (`SceneComponent.K2_GetComponentLocation` _hitcomponent))
  ;[1 1 1] Spawn Hit Impact on Enemies
  (`/Engine/EditorBlueprintResources/StandardMacros.DoOnce` false
    (:`Completed`
      (if (`ActorComponent.ComponentHasTag` OtherComp "Enemy")
        (bind _asenemy_mesh_bp (cast `/Game/VFXApprentice/Blueprints/Characters/EnemyMesh_BP` _hitactor))
        (`/Game/VFXApprentice/Blueprints/Characters/EnemyMesh_BP.ApplyHitForce` _asenemy_mesh_bp _returnvalue _ragdollforce)
        (bind _asparticle_system (cast `ParticleSystem` _impact_fx)
          (:`then`
            (bind _returnvalue_2 (`GameplayStatics.SpawnEmitterAtLocation` _asparticle_system _returnvalue))
            (set `self.ImpactFX` _returnvalue_2))
          (:`CastFailed`
            (bind _returnvalue_3 (`NiagaraFunctionLibrary.SpawnSystemAtLocation` (cast `NiagaraSystem` _impact_fx :!pure true) _returnvalue))
            (set `self.ImpactFXNiagara` _returnvalue_3)))))))

(fn `UserConstructionScript`)