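; Spawns the particle actors for the side-scroller player's active ranged, melee or instant spell.
; Wind-up spawns a stored effect actor for ranged and instant spells, destroyed on cast.
; On cast, ranged projectiles launch from CastSocket along Y by facing, and melee effects attach to the pawn.
; Instant spells appear at the Y/Z point hit by a mouse-cursor line trace, keeping them in the side-scroller plane.
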(event `OnSpellCast`
  (bind _playerpawn (`self.PlayerPawn`))
  ;[1 1 1] Spawn Spell Actors on Spell Cast
  (switch `/Game/VFXApprentice/Blueprints/SpellData/SpellsType_Enum` (`/Game/VFXApprentice/Blueprints/Characters/SideScroller_Player_BP.ActiveSpellType` (`self.PlayerPawn`))
    (:`NewEnumerator0`
      (`|SpawnActorFromClass` "/Game/VFXApprentice/Blueprints/SpellData/ProjectileParticle_BP.ProjectileParticle_BP_C" (`KismetMathLibrary.MakeTransform` (`SceneComponent.GetSocketLocation` (`Character.Mesh` (`self.PlayerPawn`)) "CastSocket") (`KismetMathLibrary.MakeRotFromX` (`KismetMathLibrary.MakeVector` 0.0 (`KismetMathLibrary.SelectFloat` -1.0 1.0 (`/Game/VFXApprentice/Blueprints/Characters/SideScroller_Player_BP.FacingRIght?` (`self.PlayerPawn`)))))) "Undefined" "OverrideRootScale" null (`/Game/VFXApprentice/Blueprints/Characters/SideScroller_Player_BP.ActiveRangedSpell` (`self.PlayerPawn`)) null)
      (`self.DestroyWindUp`))
    (:`NewEnumerator1`
      (bind _returnvalue (`|SpawnActorFromClass` "/Game/VFXApprentice/Blueprints/SpellData/MeleeParticle_BP.MeleeParticle_BP_C" (`KismetMathLibrary.MakeTransform` (`self.K2_GetActorLocation` (`self.PlayerPawn`))) "Undefined" "OverrideRootScale" null (`/Game/VFXApprentice/Blueprints/Characters/SideScroller_Player_BP.ActiveMeleeSpell` _playerpawn) (`Character.Mesh` _playerpawn) _playerpawn null))
      (`self.K2_AttachToActor` _returnvalue (`self.PlayerPawn`) "None" "KeepWorld" "KeepWorld" "KeepRelative" true))
    (:`NewEnumerator2`
      (bind _mouselocationworld (`self.FindMouseWorldLocation`))
      (`|SpawnActorFromClass` "/Game/VFXApprentice/Blueprints/SpellData/InstantParticle_BP.InstantParticle_BP_C" (`KismetMathLibrary.MakeTransform` (`KismetMathLibrary.MakeVector` 0.0 (.y _mouselocationworld) (.z _mouselocationworld))) "Undefined" "OverrideRootScale" null (`/Game/VFXApprentice/Blueprints/Characters/SideScroller_Player_BP.ActiveInstantSpell` (`self.PlayerPawn`)) (`self.PlayerPawn`) null)
      (`self.DestroyWindUp`))))

(event `OnSpellWIndUp`
  ;[1 1 1] Spawn Wind Up Actor on Ranged and Instant Spells
  (switch `/Game/VFXApprentice/Blueprints/SpellData/SpellsType_Enum` (`/Game/VFXApprentice/Blueprints/Characters/SideScroller_Player_BP.ActiveSpellType` (`self.PlayerPawn`))
    (:`NewEnumerator0`
      (bind _returnvalue (`|SpawnActorFromClass` "/Game/VFXApprentice/Blueprints/SpellData/WindUpParticle_BP.WindUpParticle_BP_C" (`KismetMathLibrary.MakeTransform` (`self.K2_GetActorLocation` (`self.PlayerPawn`))) "Undefined" "OverrideRootScale" null (`.WindUp_FX_61_DAD27212404FF580D037B7A503B39887` (break `/Game/VFXApprentice/Blueprints/SpellData/RangedSpell_Struct` (`/Game/VFXApprentice/Blueprints/Characters/SideScroller_Player_BP.ActiveRangedSpell` (`self.PlayerPawn`)))) (`self.PlayerPawn`) null))
      (set `self.WindUpParticle_BP` _returnvalue))
    (:`NewEnumerator2`
      (bind _returnvalue_2 (`|SpawnActorFromClass` "/Game/VFXApprentice/Blueprints/SpellData/WindUpParticle_BP.WindUpParticle_BP_C" (`KismetMathLibrary.MakeTransform` (`self.K2_GetActorLocation` (`self.PlayerPawn`))) "Undefined" "OverrideRootScale" null (`.WindUp_FX_47_DF441E3F46C84B5C66DA8B924122F938` (break `/Game/VFXApprentice/Blueprints/SpellData/InstantSpell_Struct` (`/Game/VFXApprentice/Blueprints/Characters/SideScroller_Player_BP.ActiveInstantSpell` (`self.PlayerPawn`)))) (`self.PlayerPawn`) null))
      (set `self.WindUpParticle_BP` _returnvalue_2))))

(fn `DestroyWindUp`
  (`/Engine/EditorBlueprintResources/StandardMacros.IsValid` (`self.WindUpParticle_BP`)
    (:`Is Valid`
      (`self.K2_DestroyActor` (`self.WindUpParticle_BP`)))))

(fn `FindMouseWorldLocation`
  (returns (MouseLocationWorld :type "Vector Structure"))
  (bind (_worldlocation _worlddirection) (`PlayerController.DeprojectMousePositionToWorld` (`GameplayStatics.GetPlayerController` 0)))
  (bind _outhit (`KismetSystemLibrary.LineTraceSingle` _worldlocation (+ _worldlocation (* _worlddirection 9000.0)) "TraceTypeQuery3"))
  (return (`.ImpactPoint` (`GameplayStatics.BreakHitResult` _outhit))))

(fn `UserConstructionScript`)