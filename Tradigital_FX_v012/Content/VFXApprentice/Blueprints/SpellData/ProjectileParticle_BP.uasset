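; Spell projectile actor that plays cast, missile and impact effects from its SpellToSpawn data, accepting Cascade or Niagara systems.
; BeginPlay spawns the detached cast effect, then after a delay attaches the missile effect, launches ProjectileMovement and starts a lifetime timer.
; Overlapping Enemy-tagged components spawns impacts and applies ragdoll force to EnemyMesh_BP.
; Impact or maximum distance can remove the missile effect, though this cleanup handles only the Cascade missile.
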(event `CalculateDistanceTraveled`
  ;[1 1 1] Calculate Distance Travel and Destroy If Set
  (if (> (`KismetMathLibrary.Vector_Distance` (`self.StartLocation`) (`self.K2_GetActorLocation`)) (`.MissileDestroyDistance_57_8FE3E51C488C19C7046A83A49E6F8DAC` (break `/Game/VFXApprentice/Blueprints/SpellData/RangedSpell_Struct` (`self.SpellToSpawn`))))
    (`self.DestroyMissile`)))

(event `DestroyMissile`
  (bind _missile_fx (`self.Missile_FX`))
  (`/Engine/EditorBlueprintResources/StandardMacros.IsValid` _missile_fx
    (:`Is Valid`
      (`ActorComponent.Deactivate` _missile_fx)
      (`KismetSystemLibrary.Delay` 1.0)
      (`ActorComponent.K2_DestroyComponent` _missile_fx))))

(event `DestroyActor`
  (for _array_element (`self.StandardEmitterFXs`)
    (`/Engine/EditorBlueprintResources/StandardMacros.IsValid` _array_element
      (:`Is Valid`
        (`ActorComponent.K2_DestroyComponent` _array_element))))
  (for _array_element_2 (`self.NiagaraEmitterFXs`)
    (`/Engine/EditorBlueprintResources/StandardMacros.IsValid` _array_element_2
      (:`Is Valid`
        (`ActorComponent.K2_DestroyComponent` _array_element_2))))
  (`self.DestroyMissile`)
  (`self.K2_DestroyActor`))

(event `self.ReceiveBeginPlay`
  (bind ((`WindUp_FX_61_DAD27212404FF580D037B7A503B39887` _windup_fx) (`Cast_FX_62_5D639F294CD498AA840C339CCC3419D4` _cast_fx) (`Missile_FX_63_0BDD4189403C24B82412D6B21F602E64` _missile_fx) (`Impact_FX_64_A51BFC634EE49FB0730E6FAE4CDE912A` _impact_fx) (`ImpactCollissionRadius_52_D20B595C43F181DD609801BFAAA6C545` _impactcollissionradius) (`MissileDestroyDistance_57_8FE3E51C488C19C7046A83A49E6F8DAC` _missiledestroydistance)) (break `/Game/VFXApprentice/Blueprints/SpellData/RangedSpell_Struct` (`self.SpellToSpawn`)))
  (`SphereComponent.SetSphereRadius` (`self.SpellBounds`) _impactcollissionradius true)
  (set `self.StartLocation` (`self.K2_GetActorLocation`))
  (set `self.CalculateMaxDistance` (> _missiledestroydistance 0.0))
  (`self.SpawnCast`)
  (`KismetSystemLibrary.Delay` (`.MissileSpawnDelay_34_D1B83234424AD73C1AD1ADA7659895E5` (break `/Game/VFXApprentice/Blueprints/SpellData/RangedSpell_Struct` (`self.SpellToSpawn`))))
  (`self.SpawnMissile`)
  (`ProjectileMovementComponent.SetVelocityInLocalSpace` (`self.ProjectileMovement`) (`.MissileVelocity_46_7912188242A4DB56FDA1ADABED98602D` (break `/Game/VFXApprentice/Blueprints/SpellData/RangedSpell_Struct` (`self.SpellToSpawn`))))
  (`KismetSystemLibrary.K2_SetTimerDelegate` (delegate `DestroyActor`) (`self.TimeTillDeath`)))

(event `SpawnCast`
  (bind _defaultsceneroot (`self.DefaultSceneRoot`))
  (bind ((`WindUp_FX_61_DAD27212404FF580D037B7A503B39887` _windup_fx) (`Cast_FX_62_5D639F294CD498AA840C339CCC3419D4` _cast_fx)) (break `/Game/VFXApprentice/Blueprints/SpellData/RangedSpell_Struct` (`self.SpellToSpawn`)))
  (bind _relativerotation (`SceneComponent.RelativeRotation` _defaultsceneroot))
  (`/Engine/EditorBlueprintResources/StandardMacros.IsValid` _cast_fx
    (:`Is Valid`
      (bind _asparticle_system (cast `ParticleSystem` _cast_fx)
        (:`then`
          (bind _returnvalue (`GameplayStatics.SpawnEmitterAttached` _asparticle_system _defaultsceneroot "None" (0.0 0.0 0.0) _relativerotation (1.0 1.0 1.0) "SnapToTarget"))
          (`SceneComponent.K2_DetachFromComponent` _returnvalue "KeepWorld" "KeepRelative" "KeepRelative" true)
          (`KismetArrayLibrary.Array_Add` (`self.StandardEmitterFXs`) _returnvalue))
        (:`CastFailed`
          (bind _returnvalue_2 (`NiagaraFunctionLibrary.SpawnSystemAttached` (cast `NiagaraSystem` _cast_fx :!pure true) _defaultsceneroot "None" (0.0 0.0 0.0) _relativerotation "SnapToTarget" true))
          (`SceneComponent.K2_DetachFromComponent` _returnvalue_2 "KeepWorld" "KeepRelative" "KeepRelative" true)
          (`KismetArrayLibrary.Array_Add` (`self.NiagaraEmitterFXs`) _returnvalue_2))))))

(event `SpawnMissile`
  (bind _defaultsceneroot (`self.DefaultSceneRoot`))
  (bind ((`Missile_FX_63_0BDD4189403C24B82412D6B21F602E64` _missile_fx)) (break `/Game/VFXApprentice/Blueprints/SpellData/RangedSpell_Struct` (`self.SpellToSpawn`)))
  ;[1 1 1] Spawn Missile Particle
  (bind _asparticle_system (cast `ParticleSystem` _missile_fx)
    (:`then`
      (bind _returnvalue (`GameplayStatics.SpawnEmitterAttached` _asparticle_system _defaultsceneroot "None" (0.0 0.0 0.0) (struct) (1.0 1.0 1.0) "SnapToTarget"))
      (set `self.Missile_FX` _returnvalue))
    (:`CastFailed`
      (bind _returnvalue_2 (`NiagaraFunctionLibrary.SpawnSystemAttached` (cast `NiagaraSystem` _missile_fx :!pure true) _defaultsceneroot "None" (0.0 0.0 0.0) (struct) "SnapToTarget" true))
      (set `self.MissileFXNiagara` _returnvalue_2))))

(event `self.ReceiveTick`
  (params (DeltaSeconds :type "Float (single-precision)"))
  (if (`self.CalculateMaxDistance`)
    (`self.CalculateDistanceTraveled`)))

(event `self.SpellBounds.OnComponentBeginOverlap`
  (params (OverlappedComponent :type "PrimitiveComponent Object Reference") (OtherActor :type "Actor Object Reference") (OtherComp :type "PrimitiveComponent Object Reference") (OtherBodyIndex :type Integer) (bFromSweep :type Boolean) (SweepResult :type "HitResult Structure (by ref)"))
  (bind (_bblockinghit _binitialoverlap _time _distance _location _impactpoint _normal _impactnormal _physmat _hitactor _hitcomponent) (`GameplayStatics.BreakHitResult` SweepResult))
  (bind ((`Impact_FX_64_A51BFC634EE49FB0730E6FAE4CDE912A` _impact_fx)) (break `/Game/VFXApprentice/Blueprints/SpellData/RangedSpell_Struct` (`self.SpellToSpawn`)))
  (bind ((`MissileDestroyOnImpact?_44_8B37226A4F06FC8EC494B49D8C23B781` _missiledestroyonimpact_) (`RagdollForce_55_8DE5C354496C538132A967B5C4FE7D7B` _ragdollforce)) (break `/Game/VFXApprentice/Blueprints/SpellData/RangedSpell_Struct` (`self.SpellToSpawn`)))
  (bind _returnvalue (`SceneComponent.K2_GetComponentLocation` _hitcomponent))
  ;[1 1 1] Spawn Impact Particle on Enemys
  (if (`ActorComponent.ComponentHasTag` OtherComp "Enemy")
    (bind _asparticle_system (cast `ParticleSystem` _impact_fx)
      (:`then`
        (bind _returnvalue_2 (`GameplayStatics.SpawnEmitterAtLocation` _asparticle_system _returnvalue))
        (`KismetArrayLibrary.Array_Add` (`self.StandardEmitterFXs`) _returnvalue_2))
      (:`CastFailed`
        (`NiagaraFunctionLibrary.SpawnSystemAtLocation` (cast `NiagaraSystem` _impact_fx :!pure true) _returnvalue)
        (`KismetArrayLibrary.Array_Add` (`self.NiagaraEmitterFXs`))))
    (if _missiledestroyonimpact_
      (`self.DestroyMissile`))
    (bind _asenemy_mesh_bp (cast `/Game/VFXApprentice/Blueprints/Characters/EnemyMesh_BP` _hitactor))
    (`/Game/VFXApprentice/Blueprints/Characters/EnemyMesh_BP.ApplyHitForce` _asenemy_mesh_bp _returnvalue _ragdollforce)))

(fn `UserConstructionScript`)